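; BP_ShooterHUD is the HUD that draws a dynamic, spreading crosshair at the screen center for the shooter character.
; It caches the player pawn as BP_ShooterCharacter on BeginPlay and retries the cast in DrawHUD if that reference is invalid.
; Each DrawHUD reads the character's crosshair multiplier, scales it by the max spread, and offsets four directional textures outward from the center.
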(event `self.ReceiveBeginPlay`
  (`/Engine/EditorBlueprintResources/StandardMacros.IsValid` (`self.ShooterCharater`)
    (:`Is Not Valid`
      (bind _asbp_shooter_character (cast `/Game/_Game/Character/BP_ShooterCharacter` (`GameplayStatics.GetPlayerPawn` 0)))
      (set `self.ShooterCharater` _asbp_shooter_character))))

(event `self.ReceiveDrawHUD`
  (params (SizeX :type Integer) (SizeY :type Integer))
  (bind (_x _y) (`KismetMathLibrary.BreakVector2D` (`self.CrosshairBaseCenter`)))
  (bind (_x_2 _y_2) (`KismetMathLibrary.BreakVector2D` (`self.CrosshairBaseCenter`)))
  (bind (_x_3 _y_3) (`KismetMathLibrary.BreakVector2D` (`self.CrosshairBaseCenter`)))
  (bind (_x_4 _y_4) (`KismetMathLibrary.BreakVector2D` (`self.CrosshairBaseCenter`)))
  (bind (_x_5 _y_5) (`KismetMathLibrary.BreakVector2D` (`self.ScreenCenter`)))
  (set `self.ScreenCenter` (`KismetMathLibrary.MakeVector2D` (`KismetMathLibrary.Conv_IntToDouble` (/ SizeX 2)) (`KismetMathLibrary.Conv_IntToDouble` (/ SizeY 2))))
  (`/Engine/EditorBlueprintResources/StandardMacros.IsValid` (`self.ShooterCharater`)
    (:`Is Valid`
      _)
    (:`Is Not Valid`
      (bind _asbp_shooter_character (cast `/Game/_Game/Character/BP_ShooterCharacter` (`GameplayStatics.GetPlayerPawn` 0)))
      (set `self.ShooterCharater` _asbp_shooter_character)))
  (set `self.CrosshairMultiplayer` (`ShooterCharacter.GetCrosshairMultiplier` (`self.ShooterCharater`)))
  (set `self.CrosshairBaseCenter` (`KismetMathLibrary.MakeVector2D` (- _x_5 (`self.Crosshar Halfwidth`)) (- _y_5 (`self.Crosshar Halfheight`))))
  (`self.DrawTexture` "/Game/_Game/HUD/Crosshair/Crosshair_Quad_9_Bottom.Crosshair_Quad_9_Bottom" _x_2 (+ _y_2 (* (`self.CrosshairMultiplayer`) (`self.CrosshairSpreadMax`))) 64.0 64.0 0.0 0.0 1.0 1.0)
  (`self.DrawTexture` "/Game/_Game/HUD/Crosshair/Crosshair_Quad_9_Top.Crosshair_Quad_9_Top" _x_4 (- _y_4 (* (`self.CrosshairMultiplayer`) (`self.CrosshairSpreadMax`))) 64.0 64.0 0.0 0.0 1.0 1.0)
  (`self.DrawTexture` "/Game/_Game/HUD/Crosshair/Crosshair_Quad_9_Right.Crosshair_Quad_9_Right" (+ _x (* (`self.CrosshairMultiplayer`) (`self.CrosshairSpreadMax`))) _y 64.0 64.0 0.0 0.0 1.0 1.0)
  (`self.DrawTexture` "/Game/_Game/HUD/Crosshair/Crosshair_Quad_9_Left.Crosshair_Quad_9_Left" (- _x_3 (* (`self.CrosshairMultiplayer`) (`self.CrosshairSpreadMax`))) _y_3 64.0 64.0 0.0 0.0 1.0 1.0))

(fn `UserConstructionScript`)